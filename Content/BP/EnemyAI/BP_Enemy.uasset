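; Patrolling enemy that catches an undisguised player and ends the attempt.
; It moves through the Waypoints array with AI MoveTo, pausing briefly at each, and loops back to index 1 rather than 0.
; When an undisguised BP_Character overlaps its Trigger, it disables the player's movement, updates the objective, gives chase and fades the screen out before opening the "Base" level.
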(event OnComponentBeginOverlap(Trigger)
  (params (OverlappedComponent :type Primitive%20Component%20Object%20Reference) (OtherActor :type Actor%20Object%20Reference) (OtherComp :type Primitive%20Component%20Object%20Reference) (OtherBodyIndex :type Integer) (bFromSweep :type Boolean) (SweepResult :type Hit%20Result%20Structure%20%28by%20ref%29))
  (bind _asbp_character (Utilities|Casting|CastToBP_Character OtherActor))
  (if (not (Variables|/Game/BP/BP_Character.BP_Character_C|GetisDisguised _asbp_character))
    (Pawn|Components|CharacterMovement|SetMovementMode (Variables|/Script/Engine.Character|GetCharacterMovement _asbp_character) "MOVE_None" 0)
    (CallFunction|UpdateObjective "" 2.0)
    (CallFunction|ChasePlayer)
    (CameraFades|StartCameraFade :self (Game|GetPlayerCameraManager 0) :ToAlpha 1.0 :Duration 3.0 :bHoldWhenFinished true)
    (Utilities|FlowControl|Delay 3.0)
    (Game|OpenLevel(byName) "Base")))

(event Custom|Follow%20Waypoint
  (AI|AIMoveTo self "0, 0, 0" (Utilities|Array|Get(acopy) (Variables|Default|Getwaypoints) (Variables|Default|GetcurrentWaypoint)) 5.0 false
    (:OnSuccess
      (Math|Integer|IncrementInt (Variables|Default|GetcurrentWaypoint)
        (:%20%20
          (if (>= (Variables|Default|GetcurrentWaypoint) (Utilities|Array|Length (Variables|Default|Getwaypoints)))
            (Variables|Default|SetcurrentWaypoint 1))
          (Utilities|FlowControl|Delay 1.0)
          (CallFunction|FollowWaypoint))))))

(event Custom|Chase%20Player
  (AI|AIMoveTo self "0, 0, 0" (Game|GetPlayerCharacter 0) 5.0 false))

(event EventBeginPlay
  (CallFunction|FollowWaypoint))

(fn ConstructionScript)