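; Player character Blueprint with Enhanced Input movement and look, plus a mask the player picks up and wears as a disguise.
; Pickup scans overlapping actors for BPI_Pickup, takes the returned mesh for the held mask, and sets HasMask.
; With a mask, the stealth input flip-flops between two mask components, toggling IsDisguised and disabling movement while disguised.
; Objective text prompts the player at each step.
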(event Input|EnhancedActionEvents|EnhancedInputActionIA_Locamotion
  (params (ActionValue :type Float%20%28double-precision%29) (ElapsedSeconds :type Float%20%28double-precision%29) (TriggeredSeconds :type Float%20%28double-precision%29) (InputAction :type Input%20Action%20Object%20Reference :default "/Game/BP/UI/IO/IA_Locamotion.IA_Locamotion"))
  ;[0.15 0.15 0.15 0.5] Basic Features
  (Pawn|Input|AddMovementInput (Transformation|GetActorForwardVector) ActionValue false))

(event Input|EnhancedActionEvents|EnhancedInputActionIA_LookH
  (params (ActionValue :type Float%20%28double-precision%29) (ElapsedSeconds :type Float%20%28double-precision%29) (TriggeredSeconds :type Float%20%28double-precision%29) (InputAction :type Input%20Action%20Object%20Reference :default "/Game/BP/UI/IO/IA_LookH.IA_LookH"))
  ;[0.15 0.15 0.15 0.5] Basic Features
  (Pawn|Input|AddControllerYawInput ActionValue))

(event Input|EnhancedActionEvents|EnhancedInputActionIA_LookV
  (params (ActionValue :type Float%20%28double-precision%29) (ElapsedSeconds :type Float%20%28double-precision%29) (TriggeredSeconds :type Float%20%28double-precision%29) (InputAction :type Input%20Action%20Object%20Reference :default "/Game/BP/UI/IO/IA_LookV.IA_LookV"))
  ;[0.15 0.15 0.15 0.5] Basic Features
  (Pawn|Input|AddControllerPitchInput ActionValue))

(event Input|EnhancedActionEvents|EnhancedInputActionIA_Strafe
  (params (ActionValue :type Float%20%28double-precision%29) (ElapsedSeconds :type Float%20%28double-precision%29) (TriggeredSeconds :type Float%20%28double-precision%29) (InputAction :type Input%20Action%20Object%20Reference :default "/Game/BP/UI/IO/IA_Strafe.IA_Strafe"))
  ;[0.15 0.15 0.15 0.5] Basic Features
  (Pawn|Input|AddMovementInput (Transformation|GetActorRightVector) ActionValue false))

(event Input|EnhancedActionEvents|EnhancedInputActionIA_Pickup
  (params (ActionValue :type Boolean) (ElapsedSeconds :type Float%20%28double-precision%29) (TriggeredSeconds :type Float%20%28double-precision%29) (InputAction :type Input%20Action%20Object%20Reference :default "/Game/BP/UI/IO/IA_Pickup.IA_Pickup"))
  (for _array_element (Collision|GetOverlappingActors 0 :!class /Script/Engine.Actor)
    (if (Utilities|DoesObjectImplementInterface _array_element "/Game/BP/Stealth/BPI_Pickup.BPI_Pickup_C")
      (bind _staticmesh (Class|BPIPickup|Pickup(Message) _array_element))
      (Components|StaticMesh|SetStaticMesh (Variables|Default|GetMask) _staticmesh)
      (Rendering|SetVisibility (Variables|Default|GetMask) true false)
      (Variables|Default|SetisDisguised false)
      (Variables|Default|SethasMask true)
      (CallFunction|UpdateObjective "Press SPACE to use the mask. You can't move with the mask on." 6.0))))

(event Input|EnhancedActionEvents|EnhancedInputActionIA_Stealth
  (params (ActionValue :type Boolean) (ElapsedSeconds :type Float%20%28double-precision%29) (TriggeredSeconds :type Float%20%28double-precision%29) (InputAction :type Input%20Action%20Object%20Reference :default "/Game/BP/UI/IO/IA_Stealth.IA_Stealth"))
  (:Started
    (if (Variables|Default|GethasMask)
      (Utilities|FlowControl|FlipFlop
        (:A
          (Rendering|SetVisibility (Variables|Default|GetMask) false false)
          (Rendering|SetVisibility (Variables|Default|GetMask2) true false)
          (Pawn|Components|CharacterMovement|SetMovementMode (Variables|Character|GetCharacterMovement) "MOVE_None" 0)
          (Variables|Default|SetisDisguised true))
        (:B
          (Rendering|SetVisibility (Variables|Default|GetMask2) false false)
          (Rendering|SetVisibility (Variables|Default|GetMask) true false)
          (Pawn|Components|CharacterMovement|SetMovementMode (Variables|Character|GetCharacterMovement) "MOVE_Walking" 0)
          (Variables|Default|SetisDisguised false)))
      (else
        (CallFunction|UpdateObjective "Pickup the mask!" 2.0)))))

(event EventBeginPlay
  ;[0.15 0.15 0.15 0.5] Establish IMC Mapping
  (Input|AddMappingContext (PlayerController|LocalPlayerSubsystems|GetEnhancedInputLocalPlayerSubsystem (Game|GetPlayerController 0)) "/Game/BP/UI/IO/IMC_baseCharacter.IMC_baseCharacter" 0 "(bIgnoreAllPressedKeysUntilRelease=True,bForceImmediately=False,bNotifyUserSettings=False)"))

(fn ConstructionScript)