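; BP_LevelCompleteVolume is a trigger volume that ends the level with a win when BP_Character overlaps it.
; It also starts a 2D background sound on BeginPlay and keeps the reference so it can stop it later.
; On overlap it swaps that sound for win music, starts a held camera fade-out, shows a win objective message, then opens the "Base" level after a delay matching the fade.
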(event OnComponentBeginOverlap(Trigger)
  (params (OverlappedComponent :type Primitive%20Component%20Object%20Reference) (OtherActor :type Actor%20Object%20Reference) (OtherComp :type Primitive%20Component%20Object%20Reference) (OtherBodyIndex :type Integer) (bFromSweep :type Boolean) (SweepResult :type Hit%20Result%20Structure%20%28by%20ref%29))
  (Utilities|Casting|CastToBP_Character OtherActor)
  (Audio|Components|Audio|Stop (Variables|Default|GetPlayingBGSound_0))
  (Audio|PlaySound2D "/Game/Audio/WinBackgroundMusic.WinBackgroundMusic" 1.0 1.0 0.0 0 0)
  (CameraFades|StartCameraFade :self (Game|GetPlayerCameraManager 0) :ToAlpha 1.0 :Duration 3.0 :bHoldWhenFinished true)
  (CallFunction|UpdateObjective "You Win!!!" 2.0)
  (Utilities|FlowControl|Delay 3.0)
  (Game|OpenLevel(byName) "Base"))

(event EventBeginPlay
  (bind _returnvalue (Audio|SpawnSound2D (Variables|Default|GetSound) 1.0 1.0 0.0 0))
  (Variables|Default|SetPlayingBGSound_0 _returnvalue))

(fn ConstructionScript)