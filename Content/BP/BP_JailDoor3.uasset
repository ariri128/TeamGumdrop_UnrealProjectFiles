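; BP_JailDoor3 is a jail door that raises its bars when the player character enters its trigger with enough items collected.
; CollectItem increments a counter, which the trigger overlap compares against MaxNumItems after casting the overlapping actor to BP_Character.
; When the count is met, LiftBars plays a timeline that interpolates the Bars component's relative Z location to slide it upward.
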(event OnComponentBeginOverlap(Trigger)
  (params (OverlappedComponent :type Primitive%20Component%20Object%20Reference) (OtherActor :type Actor%20Object%20Reference) (OtherComp :type Primitive%20Component%20Object%20Reference) (OtherBodyIndex :type Integer) (bFromSweep :type Boolean) (SweepResult :type Hit%20Result%20Structure%20%28by%20ref%29))
  (Utilities|Casting|CastToBP_Character OtherActor)
  (if (>= (Variables|Default|GetcurrentNumItems) (Variables|Default|GetmaxNumItems))
    (CallFunction|LiftBars)))

(event Custom|Lift%20Bars
  (bind _bar_lift (Timeline|Lift%20Bar%20Anime Play)
    (:Update
      (Transformation|SetRelativeLocation (Variables|Default|GetBars) (Math|Vector|MakeVector 0.0 0.0 (Math|Float|Lerp 0.0 3.5e+02 _bar_lift)) false false))))

(event Custom|Collect%20Item
  (Math|Integer|IncrementInt (Variables|Default|GetcurrentNumItems)))

(fn ConstructionScript)