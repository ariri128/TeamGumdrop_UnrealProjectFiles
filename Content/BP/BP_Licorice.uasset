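; Licorice actor that builds a bendable strand by tiling a licorice static mesh along an editable spline.
; The construction script derives the segment count from spline length and the mesh's X bounds, then adds a spline mesh component per segment with a configurable forward axis.
; GetLocAndTan supplies each segment's local endpoints and tangents, clamping tangent size to the mesh length.
; The event graph holds no active logic.
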(event EventBeginPlay)

(event Collision|EventActorBeginOverlap
  (params (OtherActor :type Actor%20Object%20Reference)))

(event EventTick
  (params (DeltaSeconds :type Float%20%28single-precision%29)))

(fn ConstructionScript
  (bind _licorice (Variables|Default|GetLicorice))
  (bind _returnvalue (StaticMesh|GetBoundingBox _licorice))
  (Variables|Default|SetMeshLenth (.x (- (.max _returnvalue) (.min _returnvalue))))
  (for _index (range 0 (Math|Float|Truncate (/ (Spline|GetSplineLength (Variables|Default|GetSpline)) (Variables|Default|GetMeshLenth))))
    (Variables|Default|SetIndex _index)
    (bind _returnvalue_2 (AddComponent|AddSplineMeshComponent false))
    (Components|StaticMesh|SetStaticMesh _returnvalue_2 (Variables|Default|GetLicorice))
    (SplineMesh|SetForwardAxis _returnvalue_2 (Variables|Default|GetIn%20Forward%20Axis) true)
    (bind (_returnvalue_3 _returnvalue2) (CallFunction|GetLocandTan (Variables|Default|GetIndex)))
    (bind (_returnvalue_4 _returnvalue2_2) (CallFunction|GetLocandTan (+ (Variables|Default|GetIndex) 1)))
    (SplineMesh|SetStartandEnd _returnvalue_2 _returnvalue_3 _returnvalue2 _returnvalue_4 _returnvalue2_2 true :!class /Script/Engine.SplineMeshComponent)))

(fn GetLocandTan
  (params (A :type Integer))
  (bind _spline (Variables|Default|GetSpline))
  (bind _meshlenth (Variables|Default|GetMeshLenth))
  (bind _returnvalue (* A _meshlenth))
  (return (Spline|GetLocationatDistanceAlongSpline _spline _returnvalue "Local") (Math|Vector|ClampVectorSize (Spline|GetTangentatDistanceAlongSpline _spline _returnvalue "Local") 0.0 (Variables|Default|GetMeshLenth))))